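; Player controller for the samurai game, handling camera, combat inputs, pause menu, danger-widget visibility and a toggled enemy lock-on.
; Attack, avoid and defense set the pawn's InputType, with a short timer switching the defense state while held.
; In lock-on, horizontal mouse input rotates a virtual aim line instead of the view.
; Each tick, a capsule trace along it picks the best-aligned visible enemy, updates target markers and drives BPRotateActor.
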(event Custom|CustomEvent_0
  (Variables|/Game/Samurai/Charactor/BaseBluePrints/BP_BaseCharactor.BP_BaseCharactor_C|SetInputType (Variables|Ref|GetPlayerPawn) "NewEnumerator2"))

(event Custom|ShowImage
  (Widget|SetVisibility (Variables|Default|GetAs%20WB%20Danger) "Visible"))

(event Custom|HideImage
  (Widget|SetVisibility (Variables|Default|GetAs%20WB%20Danger) "Hidden"))

(event EventBeginPlay
  (Utilities|IsValid (Variables|Ref|GetPlayerPawn)
    (:Is%20Not%20Valid
      (bind _asbp_charactor (Utilities|Casting|CastToBP_Charactor (Game|Player|GetPlayerPawn 0)))
      (Variables|Ref|SetPlayerPawn _asbp_charactor))))

(event EventTick
  (params (DeltaSeconds :type Float%20%28single-precision%29))
  (Variables|Default|SetDelta%20Seconds DeltaSeconds)
  (Utilities|FlowControl|Sequence
    (:then_0
      (|Arm))
    (:then_1
      (|GetUMG))))

(event Input|ActionEvents|InputActionMenu
  (params (Key :type Key%20Structure :default "None"))
  (bind _self self)
  (:Pressed
    (Game|SetGamePaused true)
    (bind _returnvalue (UserInterface|CreateWidget "/Game/Samurai/Interface/SystemUI/UI_Menu.UI_Menu_C"))
    (UserInterface|Viewport|AddtoViewport _returnvalue 0)
    (Variables|/Script/Engine.PlayerController|SetbShowMouseCursor _self true)
    (Input|SetInputModeGameandUI _self _returnvalue "DoNotLock" true)))

(event Input|ActionEvents|InputActionAvoid
  (params (Key :type Key%20Structure :default "None"))
  (:Pressed
    (Variables|/Game/Samurai/Charactor/BaseBluePrints/BP_BaseCharactor.BP_BaseCharactor_C|SetInputType (Variables|Ref|GetPlayerPawn) "NewEnumerator7"))
  (:Released
    (Variables|/Game/Samurai/Charactor/BaseBluePrints/BP_BaseCharactor.BP_BaseCharactor_C|SetInputType (Variables|Ref|GetPlayerPawn) "NewEnumerator0")))

(event Input|ActionEvents|InputActionArm
  (params (Key :type Key%20Structure :default "None"))
  (:Pressed
    (if (Variables|Default|GetIsArmModel)
      (Variables|Default|SetIsArmModel false)
      (else
        (Variables|Default|SetIsArmModel true)))))

(event Input|ActionEvents|InputActionAttack
  (params (Key :type Key%20Structure :default "None"))
  (:Pressed
    (Variables|/Game/Samurai/Charactor/BaseBluePrints/BP_BaseCharactor.BP_BaseCharactor_C|SetInputType (Variables|Ref|GetPlayerPawn) "NewEnumerator1"))
  (:Released
    (Variables|/Game/Samurai/Charactor/BaseBluePrints/BP_BaseCharactor.BP_BaseCharactor_C|SetInputType (Variables|Ref|GetPlayerPawn) "NewEnumerator0")))

(event Input|ActionEvents|InputActionDefense
  (params (Key :type Key%20Structure :default "None"))
  (bind _playerpawn (Variables|Ref|GetPlayerPawn))
  (:Pressed
    (Variables|/Game/Samurai/Charactor/BaseBluePrints/BP_BaseCharactor.BP_BaseCharactor_C|SetInputType (Variables|Ref|GetPlayerPawn) "NewEnumerator3")
    (bind _returnvalue (Utilities|Time|SetTimerbyEvent (delegate Custom|CustomEvent_0) 0.1))
    (Variables|Default|SetDefendHandle _returnvalue))
  (:Released
    (Variables|/Game/Samurai/Charactor/BaseBluePrints/BP_BaseCharactor.BP_BaseCharactor_C|SetInputType (Variables|Ref|GetPlayerPawn) "NewEnumerator0")
    (Utilities|Time|ClearandInvalidateTimerbyHandle (Variables|Default|GetDefendHandle))
    (Variables|/Game/Samurai/Charactor/BaseBluePrints/BP_BaseCharactor.BP_BaseCharactor_C|SetCharactorType _playerpawn "NewEnumerator0")
    (Variables|/Game/Samurai/Charactor/BaseBluePrints/BP_PlayAnimMontageComponent.BP_PlayAnimMontageComponent_C|SetBack (Variables|/Game/Samurai/Charactor/BaseBluePrints/BP_BaseCharactor.BP_BaseCharactor_C|GetBP_PlayAnimMontageComponent _playerpawn) false)))

(event Input|AxisEvents|InputAxisMouseUP/Down
  (params (AxisValue :type Float%20%28single-precision%29))
  (if (not (Variables|Default|GetIsArmModel))
    (Pawn|Input|AddControllerPitchInput (Variables|Ref|GetPlayerPawn) AxisValue)))

(event Input|AxisEvents|InputAxisMouseLeft/Right
  (params (AxisValue :type Float%20%28single-precision%29))
  (if (Variables|Default|GetIsArmModel)
    (Variables|Default|SetVirtualLine (Math|Vector|RotateVector (Variables|Default|GetVirtualLine) (Math|Rotator|MakeRotator 0.0 0.0 AxisValue)))
    (else
      (Pawn|Input|AddControllerYawInput (Variables|Ref|GetPlayerPawn) AxisValue)
      (Variables|Default|SetVirtualLine (Transformation|GetActorForwardVector (Pawn|GetController (Variables|Ref|GetPlayerPawn)))))))

(event Input|AxisEvents|InputAxisMoveForward
  (params (AxisValue :type Float%20%28single-precision%29))
  (Variables|Default|SetMoveAxis (Math|Vector2D|MakeVector2D (.x (Variables|Default|GetMoveAxis)) AxisValue)))

(event Input|AxisEvents|InputAxisMoveRight
  (params (AxisValue :type Float%20%28single-precision%29))
  (Variables|Default|SetMoveAxis (Math|Vector2D|MakeVector2D AxisValue (.y (Variables|Default|GetMoveAxis)))))

(event Input|KeyboardEvents|Q
  (params (Key :type Key%20Structure :default "None"))
  (bind _playerpawn (Variables|Ref|GetPlayerPawn))
  (:Pressed
    (Effects|SpawnEmitteratLocation "/Game/FXVillesBloodVFXPack/Particles/PS_Blood_Slice.PS_Blood_Slice" (Transformation|GetActorLocation _playerpawn) (Math|Conversions|RotationFromXVector (Math|Vector|RotateVector (Math|Vector|GetForwardVector (Variables|/Game/Samurai/Charactor/Player/Blueprints/BP_Charactor.BP_Charactor_C|GetCamera _playerpawn)) "0,-90.000000, 0")))))

(fn ConstructionScript)

(fn GetDotOfTwoActor
  (params (Player :type BP%20Charactor%20Object%20Reference) (Actor2 :type Actor%20Object%20Reference))
  (return (Math|Vector|DotProduct (Math|Vector|Normalize (Math|Vector|GetForwardVector (Variables|/Game/Samurai/Charactor/Player/Blueprints/BP_Charactor.BP_Charactor_C|GetCamera Player))) (Math|Vector|Normalize (- (Transformation|GetActorLocation Actor2) (Transformation|GetActorLocation Player))))))

(fn NewFunction0
  (bind _playerpawn (Variables|Ref|GetPlayerPawn))
  (bind _returnvalue (Transformation|GetActorLocation _playerpawn))
  (bind _output_get (Variables|Default|SetVirtualLine (Transformation|GetActorForwardVector (Pawn|GetController _playerpawn))))
  (return _returnvalue (+ _returnvalue (* _output_get 1e+03))))