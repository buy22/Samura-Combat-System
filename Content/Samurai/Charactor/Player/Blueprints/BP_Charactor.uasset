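; Samurai player character Blueprint that wires up katana damage detection, montage playback and movement input.
; On BeginPlay it registers the Katana's sockets with BPDamageCheck, hides its widget and initializes the montage component with itself.
; Tick lazily caches BP_PlayerController, then copies its MoveAxis each frame and switches the weapon damage trace on or off from the EnableDoDAmage flag.
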(event EventBeginPlay
  (Default|InitWeaponSockets (Variables|Default|GetBP_DamageCheck) (Variables|Default|GetKatana))
  (Widget|SetVisibility (UserInterface|GetWidget (Variables|Default|GetWidget)) "Hidden")
  (Default|Init (Variables|Default|GetBP_PlayAnimMontageComponent) self))

(event EventTick
  (params (DeltaSeconds :type Float%20%28single-precision%29))
  (bind _bp_damagecheck (Variables|Default|GetBP_DamageCheck))
  (Utilities|IsValid (Variables|Default|GetPlayer%20Controller)
    (:Is%20Valid
      (Variables|Default|SetMoveAxis (Variables|/Game/Samurai/Charactor/Player/Blueprints/BP_PlayerController.BP_PlayerController_C|GetMoveAxis (Variables|Default|GetPlayer%20Controller)))
      (if (Variables|Default|GetEnableDoDAmage)
        (Default|EnableTrace _bp_damagecheck)
        (else
          (Default|DisableTrace _bp_damagecheck))))
    (:Is%20Not%20Valid
      (bind _asbp_player_controller (Utilities|Casting|CastToBP_PlayerController (Pawn|GetController)))
      (Variables|Default|SetPlayer%20Controller _asbp_player_controller))))

(fn ConstructionScript
  (|CallParentFunction))